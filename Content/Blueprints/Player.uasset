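; First-person player Blueprint handling movement, mouse look with optional pitch inversion, and interaction with world objects.
; Interact line-traces a short distance from the camera and sends an interface message to the hit actor.
; A held item is put down at the impact point when the hit is a Surface.
; AssignEquippedItem sets the held item, and equip changes fire a dispatcher; construction caches the grab point transform.
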(event Custom|AssignEquippedItem
  (params (ItemToEquip :type Actor%20Object%20Reference))
  (bind _output_get (Variables|Default|SetEquippedItem ItemToEquip))
  (Default|CallItemEquippedDispatcher _output_get))

(event EventTick
  (params (DeltaSeconds :type Float%20%28single-precision%29))
  ;[1 1 1] Mouse and camera controls
  (Pawn|Input|AddControllerYawInput (Class|Actor|GetInputAxisKeyValue))
  (if (Variables|Default|GetInvertedMouse)
    (Pawn|Input|AddControllerPitchInput (Class|Actor|GetInputAxisKeyValue))
    (else
      (Pawn|Input|AddControllerPitchInput (* (Class|Actor|GetInputAxisKeyValue) -1.0)))))

(event Input|ActionEvents|InputActionInteract
  (params (Key :type Key%20Structure :default "None"))
  (bind _camera (Variables|Default|GetCamera))
  (bind _returnvalue (Transformation|GetWorldLocation _camera))
  (:Pressed
    (bind (_outhit _returnvalue_2) (Collision|LineTraceByChannel _returnvalue (+ (* (Math|Vector|GetForwardVector (Transformation|GetWorldRotation _camera)) 3e+02) _returnvalue) "TraceTypeQuery1" false 0 "Persistent"))
    (if _returnvalue_2
      ;[1 1 1] message called from actor if it implements the interact interface
      (Class|InteractionInterface|Interact(Message) (.HitActor (Collision|BreakHitResult _outhit)))
      (Utilities|IsValid (Variables|Default|GetEquippedItem)
        (:Is%20Valid
          ;[1 1 1] Call for when equpped item state change
          (Default|CallItemEquippedDispatcher (Variables|Default|GetEquippedItem))
          ;[1 1 1] Putting object down
          ;;[1 1 1] if we are holding an item and hit a surface
          (Utilities|Casting|CastToSurface (.HitActor (Collision|BreakHitResult _outhit)))
          (bind _as_interactive_object_base (Utilities|Casting|CastTo_InteractiveObjectBase (Variables|Default|GetEquippedItem)))
          (Default|OnPutDown _as_interactive_object_base (.ImpactPoint (Collision|BreakHitResult _outhit)))
          ;;[1 1 1] Sets equpped item back to null
          (Variables|Default|SetEquippedItem 0)
          (Default|CallItemEquippedDispatcher))))))

(event Input|AxisEvents|InputAxisMove_ForwardBack
  (params (AxisValue :type Float%20%28single-precision%29))
  ;[1 1 1] Player Movement
  (Pawn|Input|AddMovementInput (Transformation|GetActorForwardVector) AxisValue false))

(event Input|AxisEvents|InputAxisMove_LeftRight
  (params (AxisValue :type Float%20%28single-precision%29))
  ;[1 1 1] Player Movement
  (Pawn|Input|AddMovementInput (Transformation|GetActorRightVector) AxisValue false))

(fn ConstructionScript
  (Variables|Default|SetEquippedItemTransform (Transformation|GetWorldTransform (Variables|Default|GetObjectGrabPoint))))