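; Interactive tea cup that the player fills from a boiled kettle to make tea.
; On interact, if the player's equipped item is a boiled kettle, the cup becomes filled and the kettle is set to empty.
; When the player's equipment changes to a kettle, the kettle's state picks the "E)" prompt on the text render, either "Make tea" or "Needs boiling water".
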(event EventBeginPlay
  (|CallParentFunction) ; This node is disabled and will not be called.\nDrag off pins to build functionality.
)

(event EventTick
  (params (DeltaSeconds :type Float%20%28single-precision%29))
  (|CallParentFunction DeltaSeconds) ; This node is disabled and will not be called.\nDrag off pins to build functionality.
)

(event EventInteract
  (|CallParentFunction)
  (bind _asplayer (Utilities|Casting|CastToPlayer (Variables|Default|GetPlayer)))
  (Utilities|IsValid (Variables|/Game/Blueprints/Player.Player_C|GetEquippedItem _asplayer)
    (:Is%20Valid
      (bind _askettle_interactive (Utilities|Casting|CastToKettle_Interactive (Variables|/Game/Blueprints/Player.Player_C|GetEquippedItem _asplayer)))
      (switch Utilities|FlowControl|Switch|SwitchonInteractiveObjectState (Variables|/Game/Blueprints/InteractiveItems/Kettle_Interactive.Kettle_Interactive_C|GetKettleState _askettle_interactive)
        (:NewEnumerator2
          (Variables|Default|SetCupState "NewEnumerator1")
          (Variables|/Game/Blueprints/InteractiveItems/Kettle_Interactive.Kettle_Interactive_C|SetKettleState _askettle_interactive "NewEnumerator0"))))))

(event EventPlayerEquipChange
  (params (ItemCurrentlyEquiped :type Actor%20Object%20Reference))
  (|CallParentFunction ItemCurrentlyEquiped)
  (bind _askettle_interactive (Utilities|Casting|CastToKettle_Interactive ItemCurrentlyEquiped))
  (switch Utilities|FlowControl|Switch|SwitchonInteractiveObjectState (Variables|/Game/Blueprints/InteractiveItems/Kettle_Interactive.Kettle_Interactive_C|GetKettleState _askettle_interactive)
    (:NewEnumerator0
      (Variables|Default|SetCupStateText "Needs boiling water" :!label _label))
    (:NewEnumerator1
      (goto _label))
    (:NewEnumerator2
      (Variables|Default|SetCupStateText "Make tea")))
  (Rendering|Components|TextRender|SetText (Variables|Default|GetTextRender) (Utilities|Text|ToText(String) (Utilities|String|Append "E) " (Variables|Default|GetCupStateText)))))

(fn ConstructionScript
  (|CallParentFunction))