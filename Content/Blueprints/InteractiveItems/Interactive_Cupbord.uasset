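; Interactive cupboard whose door swings on its hinge when the player interacts, extending a parent's Interact event.
; The DoorOpen timeline drives the door's relative yaw, scaling its track by 90 degrees.
; Interact toggles the Open flag, playing the timeline when it was true and reversing it otherwise.
; BeginPlay clears the text render and also plays the timeline, so the door animates at startup.
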(event EventBeginPlay
  (|CallParentFunction)
  (Rendering|Components|TextRender|SetText (Variables|Default|GetTextRender) (Utilities|Text|ToText(String) ""))
  (bind _newtrack_0 (Timeline|DoorOpen Play)
    (:Update
      (Transformation|SetRelativeRotation (Variables|Default|GetDoor) (Math|Rotator|MakeRotator 0.0 0.0 (* _newtrack_0 9e+01)) false false))))

(event Collision|EventActorBeginOverlap
  (params (OtherActor :type Actor%20Object%20Reference))
  (|CallParentFunction OtherActor) ; This node is disabled and will not be called.\nDrag off pins to build functionality.
)

(event EventTick
  (params (DeltaSeconds :type Float%20%28single-precision%29))
  (|CallParentFunction DeltaSeconds) ; This node is disabled and will not be called.\nDrag off pins to build functionality.
)

(event EventInteract
  (|CallParentFunction)
  (if (Variables|Default|GetOpen)
    (Variables|Default|SetOpen false)
    (bind _newtrack_0 (Timeline|DoorOpen Play)
      (:Update
        (Transformation|SetRelativeRotation (Variables|Default|GetDoor) (Math|Rotator|MakeRotator 0.0 0.0 (* _newtrack_0 9e+01)) false false)))
    (else
      (Variables|Default|SetOpen true)
      (Timeline|DoorOpen Reverse))))

(fn ConstructionScript
  (|CallParentFunction))