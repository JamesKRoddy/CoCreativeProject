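; KettleBase_Interactive is an interactive kettle base on which the player can put down an equipped kettle.
; On a successful interaction while unoccupied, it checks that the player's equipped item is a Kettle_Interactive, sets KettlePlaced and calls the kettle's OnPutDown at the ObjectBase location.
; When the player's equipped item changes to a kettle, it clears KettlePlaced so the base can accept one again.
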(event EventBeginPlay
  (|CallParentFunction) ; This node is disabled and will not be called.\nDrag off pins to build functionality.
)

(event Collision|EventActorBeginOverlap
  (params (OtherActor :type Actor%20Object%20Reference))
  (|CallParentFunction OtherActor) ; This node is disabled and will not be called.\nDrag off pins to build functionality.
)

(event EventTick
  (params (DeltaSeconds :type Float%20%28single-precision%29))
  (|CallParentFunction DeltaSeconds) ; This node is disabled and will not be called.\nDrag off pins to build functionality.
)

(event EventPlayerEquipChange
  (params (ItemCurrentlyEquiped :type Actor%20Object%20Reference))
  (|CallParentFunction ItemCurrentlyEquiped)
  (Utilities|Casting|CastToKettle_Interactive ItemCurrentlyEquiped)
  (Variables|Default|SetKettlePlaced false))

(event EventSuccessfulInteract
  (if (not (Variables|Default|GetKettlePlaced))
    (bind _asplayer (Utilities|Casting|CastToPlayer (Variables|Default|GetPlayer)))
    (Utilities|IsValid (Variables|/Game/Blueprints/Player.Player_C|GetEquippedItem _asplayer)
      (:Is%20Valid
        (bind _askettle_interactive (Utilities|Casting|CastToKettle_Interactive (Variables|/Game/Blueprints/Player.Player_C|GetEquippedItem _asplayer)))
        (Variables|Default|SetKettlePlaced true)
        (Default|OnPutDown _askettle_interactive (Transformation|GetWorldLocation (Variables|Default|GetObject%20Base)))))))

(fn ConstructionScript
  (|CallParentFunction))