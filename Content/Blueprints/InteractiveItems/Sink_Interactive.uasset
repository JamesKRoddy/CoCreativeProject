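; Interactive sink item that fills the player's kettle.
; On Interact, after the parent logic runs, it casts the player's equipped item to Kettle_Interactive.
; If that kettle's state is Empty, it switches it to Filled; any other state or item is left untouched.
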(event EventBeginPlay
  (|CallParentFunction) ; This node is disabled and will not be called.\nDrag off pins to build functionality.
)

(event Collision|EventActorBeginOverlap
  (params (OtherActor :type Actor%20Object%20Reference))
  (|CallParentFunction OtherActor) ; This node is disabled and will not be called.\nDrag off pins to build functionality.
)

(event EventTick
  (params (DeltaSeconds :type Float%20%28single-precision%29))
  (|CallParentFunction DeltaSeconds) ; This node is disabled and will not be called.\nDrag off pins to build functionality.
)

(event EventInteract
  (|CallParentFunction)
  (bind _asplayer (Utilities|Casting|CastToPlayer (Variables|Default|GetPlayer)))
  (bind _askettle_interactive (Utilities|Casting|CastToKettle_Interactive (Variables|/Game/Blueprints/Player.Player_C|GetEquippedItem _asplayer)))
  (switch Utilities|FlowControl|Switch|SwitchonInteractiveObjectState (Variables|/Game/Blueprints/InteractiveItems/Kettle_Interactive.Kettle_Interactive_C|GetKettleState _askettle_interactive)
    (:NewEnumerator0
      (Variables|/Game/Blueprints/InteractiveItems/Kettle_Interactive.Kettle_Interactive_C|SetKettleState _askettle_interactive "NewEnumerator1"))))

(fn ConstructionScript
  (|CallParentFunction))