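; Base actor for interactive items, with a floating "E)" prompt and optional pickup into the player's hands.
; The prompt faces the player within range and updates on the player's equip dispatcher to show interaction or failure text.
; Interact checks any required equipped item, calling success or failure hooks, then pickupable items attach to the grab point if nothing is equipped.
; OnPutDown detaches and teleports the item to a target position.
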(event Custom|OnPickup
  (bind _asplayer (Utilities|Casting|CastToPlayer (Variables|Default|GetPlayer)))
  (Utilities|IsValid (Variables|/Game/Blueprints/Player.Player_C|GetEquippedItem _asplayer)
    (:Is%20Not%20Valid
      (Variables|Default|SetBeingCarried true)
      (Transformation|AttachComponentToComponent (Variables|Default|GetObject%20Base) (Variables|/Game/Blueprints/Player.Player_C|GetObjectGrabPoint _asplayer) "None" "SnapToTarget" "KeepRelative" "KeepRelative" true)
      (Default|AssignEquippedItem _asplayer self)
      (Variables|/Game/Blueprints/Player.Player_C|SetEquippedItem _asplayer self)
      (Rendering|Components|TextRender|SetText (Variables|Default|GetTextRender) (Class|KismetTextLibrary|GetEmptyText)))))

(event Custom|OnPutDown
  (params (TargetPosition :type Vector))
  (Transformation|DetachFromActor "KeepRelative" "KeepRelative" "KeepRelative")
  (Transformation|SetActorLocation TargetPosition false true)
  (Variables|Default|SetBeingCarried false))

(event Custom|PlayerEquipChange
  (params (ItemCurrentlyEquiped :type Actor%20Object%20Reference))
  (bind _itemrequiredforinteraction (Variables|Default|GetItemRequiredForInteraction))
  (bind _textrender (Variables|Default|GetTextRender))
  (if (not (Variables|Default|GetBeingCarried))
    (Utilities|IsValid _itemrequiredforinteraction
      (:Is%20Valid
        (if (== _itemrequiredforinteraction ItemCurrentlyEquiped)
          ;[1 1 1] Can Interact text
          (Rendering|Components|TextRender|SetText (Variables|Default|GetTextRender) (Utilities|Text|ToText(String) (Utilities|String|Append "E) " (Variables|Default|GetInteractionText))) :!label _label)
          (else
            (Development|PrintString (Utilities|GetDisplayName (Variables|Default|GetObject%20Base)))
            (if (Utilities|Array|IsEmpty (Variables|Default|GetFailedInteractionText))
              (Rendering|Components|TextRender|SetText _textrender (Utilities|Text|ToText(String) ""))
              (else
                ;[1 1 1] Cant Interact text
                (Rendering|Components|TextRender|SetText _textrender (Utilities|Text|ToText(String) (Utilities|String|Append "E) " (Variables|Default|GetFailedInteractionText)))))))))
      (:Is%20Not%20Valid
        (goto _label)))))

(event EventBeginPlay
  (bind _returnvalue (Actor|GetActorOfClass "/Game/Blueprints/Player.Player_C"))
  (bind _output_get (Variables|Default|SetPlayer _returnvalue))
  (bind _asplayer (Utilities|Casting|CastToPlayer _output_get))
  (EventDispatchers|BindEventtoItemEquippedDispatcher _asplayer (delegate Custom|PlayerEquipChange))
  (CallFunction|PlayerEquipChange))

(event Collision|EventActorBeginOverlap
  (params (OtherActor :type Actor%20Object%20Reference)))

(event EventTick
  (params (DeltaSeconds :type Float%20%28single-precision%29))
  (bind _scene (Variables|Default|GetScene))
  (if (not (Variables|Default|GetBeingCarried))
    (if (< (Transformation|GetDistanceTo (Variables|Default|GetPlayer)) 5e+02)
      (Rendering|SetVisibility (Variables|Default|GetTextRender) true false)
      ;[1 1 1] handles rotation of text towards player
      (Transformation|SetWorldRotation _scene (Math|Rotator|FindLookatRotation (Transformation|GetWorldLocation _scene) (+ (Transformation|GetActorLocation (Variables|Default|GetPlayer)) "0,0.000000,80.000000")) false false)
      (else
        (Rendering|SetVisibility (Variables|Default|GetTextRender) false false)))))

(event EventInteract
  ;[1 1 1] Check to see if an object is required to interact
  (if (Utilities|IsValid (Variables|Default|GetItemRequiredForInteraction))
    ;[1 1 1] Check if required item is equipped
    (bind _returnvalue (CallFunction|CanInteractCheck))
    (if _returnvalue
      (CallFunction|SuccessfulInteract)
      ;[1 1 1] Setup and equipping item
      (if (Variables|Default|GetPickUpAble) :!label _label
        (CallFunction|OnPickup))
      (else
        (CallFunction|FailedInteract)))
    (else
      (goto _label))))

(fn ConstructionScript)

(fn CanInteractCheck
  (bind _asplayer (Utilities|Casting|CastToPlayer (Variables|Default|GetPlayer)))
  (return (== (Variables|Default|GetItemRequiredForInteraction) (Variables|/Game/Blueprints/Player.Player_C|GetEquippedItem _asplayer))))