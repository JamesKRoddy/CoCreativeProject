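; InteractiveManager runs a linear sequence of interaction events driven by the items the player equips.
; It binds to the player's item-equipped dispatcher and compares the equipped item's class and interactive state against the current event.
; On a match it optionally changes a target object's state and moves it to a marker actor's location, then advances to the next event.
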(event Custom|ChangeCurrentEvent
  (params (EventIndex :type Integer))
  (if (< (Variables|Default|GetCurrentEventIndex) (Utilities|Array|Length (Variables|Default|GetInteractionEvents)))
    (Variables|Default|SetCurrentEvent (Utilities|Array|Get(acopy) (Variables|Default|GetInteractionEvents) EventIndex))))

(event Custom|CheckCustomEvent
  (params (ItemCurrentlyEquipped :type Actor%20Object%20Reference))
  (bind _currentevent (Variables|Default|GetCurrentEvent))
  (if (< (Variables|Default|GetCurrentEventIndex) (Utilities|Array|Length (Variables|Default|GetInteractionEvents)))
    (bind _asplayer (Utilities|Casting|CastToPlayer (Variables|Default|GetPlayer)))
    (Utilities|IsValid (Variables|/Game/Blueprints/Player.Player_C|GetEquippedItem _asplayer)
      (:Is%20Valid
        (if (== (Utilities|GetClass (Variables|/Game/Blueprints/Player.Player_C|GetEquippedItem _asplayer)) (Utilities|GetClass (.checkitem _currentevent)))
          (bind _as_interactive_object_base (Utilities|Casting|CastTo_InteractiveObjectBase (Variables|/Game/Blueprints/Player.Player_C|GetEquippedItem _asplayer)))
          (if (Utilities|Enum|Equal(Enum) (Variables|/Game/Blueprints/InteractiveItems/_InteractiveObjectBase._InteractiveObjectBase_C|GetInteractiveState _as_interactive_object_base) (.checkstate _currentevent))
            (if (Utilities|Enum|Equal(Enum) (.statetochange _currentevent) "NewEnumerator3")
              _
              (else
                (Variables|/Game/Blueprints/InteractiveItems/_InteractiveObjectBase._InteractiveObjectBase_C|SetInteractiveState (.objecttochange _currentevent) (.statetochange _currentevent))))
            (Utilities|IsValid (.positiontochange _currentevent)
              (:Is%20Valid
                (Development|PrintString "Moved")
                (Transformation|SetActorLocation (.objecttochange _currentevent) (.location (Transformation|GetActorTransform (.positiontochange _currentevent))) false false))
              (:Is%20Not%20Valid
                _))
            (bind _result (Math|Integer|IncrementInt (Variables|Default|GetCurrentEventIndex))
              (:%20%20
                (bind _output_get (Variables|Default|SetCurrentEventIndex _result))
                (CallFunction|ChangeCurrentEvent _output_get)))))))))

(event EventBeginPlay
  (bind _returnvalue (Actor|GetActorOfClass "/Game/Blueprints/Player.Player_C"))
  (bind _output_get (Variables|Default|SetPlayer _returnvalue))
  (bind _asplayer (Utilities|Casting|CastToPlayer _output_get))
  (EventDispatchers|BindEventtoItemEquippedDispatcher _asplayer (delegate Custom|CheckCustomEvent))
  (CallFunction|ChangeCurrentEvent (Variables|Default|GetCurrentEventIndex)))

(fn ConstructionScript)