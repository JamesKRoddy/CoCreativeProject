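; Interactive light switch that toggles an array of lights and the look of their fixture meshes when interacted with.
; BeginPlay starts everything off by hiding each light's root component and applying a glass material to the meshes.
; Interact flip-flops between showing lights with an emissive material and restoring the off state.
; The off-state material pass is chained inside the light loop, so it repeats for every light.
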(event EventBeginPlay
  (|CallParentFunction)
  (for _array_element (Variables|Default|GetLight)
    (Rendering|SetVisibility (Variables|/Script/Engine.Actor|GetRootComponent _array_element) false false)
    (for _array_element_2 (Variables|Default|GetLightMesh)
      (bind _asstatic_mesh_actor (Utilities|Casting|CastToStaticMeshActor _array_element_2))
      (Rendering|Material|SetMaterial (Variables|/Script/Engine.StaticMeshActor|GetStaticMeshComponent _asstatic_mesh_actor) (Variables|Default|GetMaterial%20Index) "/Game/Paul_Assets_Folder/70s_BathRoom/70s_shower/glass_MAT.glass_MAT"))))

(event Collision|EventActorBeginOverlap
  (params (OtherActor :type Actor%20Object%20Reference))
  (|CallParentFunction OtherActor) ; This node is disabled and will not be called.\nDrag off pins to build functionality.
)

(event EventTick
  (params (DeltaSeconds :type Float%20%28single-precision%29))
  (|CallParentFunction DeltaSeconds) ; This node is disabled and will not be called.\nDrag off pins to build functionality.
)

(event EventInteract
  (bind _light (Variables|Default|GetLight))
  (|CallParentFunction)
  (Utilities|FlowControl|FlipFlop
    (:A
      (for _array_element _light
        (Rendering|SetVisibility (Variables|/Script/Engine.Actor|GetRootComponent _array_element) true false))
      (for _array_element_2 (Variables|Default|GetLightMesh)
        (bind _asstatic_mesh_actor (Utilities|Casting|CastToStaticMeshActor _array_element_2))
        (Rendering|Material|SetMaterial (Variables|/Script/Engine.StaticMeshActor|GetStaticMeshComponent _asstatic_mesh_actor) (Variables|Default|GetMaterial%20Index) "/Game/Paul_Assets_Folder/70s_BathRoom/Light_emission_MAT.Light_emission_MAT")))
    (:B
      (for _array_element_3 _light
        (Rendering|SetVisibility (Variables|/Script/Engine.Actor|GetRootComponent _array_element_3) false false))
      (for _array_element_4 (Variables|Default|GetLightMesh)
        (bind _asstatic_mesh_actor_2 (Utilities|Casting|CastToStaticMeshActor _array_element_4))
        (Rendering|Material|SetMaterial (Variables|/Script/Engine.StaticMeshActor|GetStaticMeshComponent _asstatic_mesh_actor_2) (Variables|Default|GetMaterial%20Index) "/Game/Paul_Assets_Folder/70s_BathRoom/70s_shower/glass_MAT.glass_MAT")))))

(fn ConstructionScript
  (|CallParentFunction))